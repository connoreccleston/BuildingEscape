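; Swinging door actor that rotates open and closed in response to OnOpen and OnClose events from its DoorOpener.
; The Swing timeline plays forward to open and reverses to close, adding its OpenAngle track as yaw to the rotation cached at BeginPlay.
; A Sound event track on the same timeline plays the Doorlock sound at the door's location.
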(event OnClose(DoorOpener)
  (bind _openangle (Timeline|Swing Reverse)
    (:Update
      (Transformation|SetActorRotation (Math|Rotator|CombineRotators (Variables|Default|GetInitialRot) (Math|Rotator|MakeRotator 0.0 0.0 _openangle))))
    (:Sound
      (Audio|PlaySoundatLocation "/Game/door-lock.door-lock" (Transformation|GetActorLocation)))))

(event OnOpen(DoorOpener)
  (bind _openangle (Timeline|Swing Play)
    (:Update
      (Transformation|SetActorRotation (Math|Rotator|CombineRotators (Variables|Default|GetInitialRot) (Math|Rotator|MakeRotator 0.0 0.0 _openangle))))
    (:Sound
      (Audio|PlaySoundatLocation "/Game/door-lock.door-lock" (Transformation|GetActorLocation)))))

(event EventBeginPlay
  (Variables|Default|SetInitialRot (Transformation|GetActorRotation)))

(fn ConstructionScript)